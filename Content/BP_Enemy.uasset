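; BP_Enemy is an enemy that loses health when the third-person character enters its sphere trigger.
; On overlap, it asks the character's held item for damage against its element type.
; It scales that integer damage from percent to a fraction, subtracts it from Health and prints the result for debugging.
; It has no death handling, and construction, BeginPlay and Tick do nothing.
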(event `self.ReceiveBeginPlay`)

(event `self.Sphere.OnComponentBeginOverlap`
  (params (OverlappedComponent :type "PrimitiveComponent Object Reference") (OtherActor :type "Actor Object Reference") (OtherComp :type "PrimitiveComponent Object Reference") (OtherBodyIndex :type Integer) (bFromSweep :type Boolean) (SweepResult :type "HitResult Structure (by ref)"))
  (bind _asbp_third_person_character (cast `/Game/ThirdPerson/Blueprints/BP_ThirdPersonCharacter` OtherActor))
  (bind _damage (`/Game/BP_Item.GetDamage` (`/Game/ThirdPerson/Blueprints/BP_ThirdPersonCharacter.heldItem` _asbp_third_person_character) (`self.ElemType`)))
  (bind _output_get (set `self.Health` (- (`self.Health`) (* (`KismetMathLibrary.Conv_IntToDouble` _damage) 0.01))))
  (`KismetSystemLibrary.PrintString` (`KismetStringLibrary.Concat_StrStr` "heaalth is now" (`KismetStringLibrary.Conv_DoubleToString` _output_get))))

(fn `UserConstructionScript`)