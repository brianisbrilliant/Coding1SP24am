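; BP_Key is a collectible key pickup for the third-person player character.
; When its sphere component is hit by BP_ThirdPersonCharacter, it increments that character's TotalKeys and prints the new count for debugging.
; It then plays a pickup sound with randomized pitch at its location and destroys itself.
; Pickup relies on a blocking hit event; the overlap event is unused.
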(event `self.Sphere.OnComponentHit`
  (params (HitComponent :type "PrimitiveComponent Object Reference") (OtherActor :type "Actor Object Reference") (OtherComp :type "PrimitiveComponent Object Reference") (NormalImpulse :type "Vector Structure") (Hit :type "HitResult Structure (by ref)"))
  (bind _asbp_third_person_character (cast `/Game/ThirdPerson/Blueprints/BP_ThirdPersonCharacter` OtherActor)) ; Was it the player that hit us?
  (bind _totalkeys (`/Game/ThirdPerson/Blueprints/BP_ThirdPersonCharacter.TotalKeys` _asbp_third_person_character))
  (`/Engine/EditorBlueprintResources/StandardMacros.IncrementInt` _totalkeys ; Add one to the player's \ntotalKeys variable.
    (:`  `
      (`KismetSystemLibrary.PrintString` (`KismetStringLibrary.Concat_StrStr` "TotalKeys = " (`KismetStringLibrary.Conv_IntToString` _totalkeys)))
      (`GameplayStatics.SpawnSoundAtLocation` "/Game/Audio/Pickup_Coin31_Cue.Pickup_Coin31_Cue" (`SceneComponent.K2_GetComponentLocation` (`self.DefaultSceneRoot`)) (struct) 1.0 (`KismetMathLibrary.RandomFloatInRange` 0.8 1.2) 0.0 null null)
      (`self.K2_DestroyActor`) ; Destroy the key because\nit has been picked up.
    )))

(fn `UserConstructionScript`)