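; BP_Item is an item actor that gives itself a random person's name and announces it when play begins.
; The construction script replaces the default name "Item" with a random pick from a small hard-coded list, leaving any other name untouched.
; BeginPlay prints a greeting with that name to the screen; overlap and tick events are unused.
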(event `self.ReceiveBeginPlay`
  (`KismetSystemLibrary.PrintString` (`KismetStringLibrary.Concat_StrStr` "Hello! My name is " (`self.Name`))))

(fn `UserConstructionScript`
  (bind _array (`|MakeArray` "Brian" "Gabe" "Robert" "Jalen"))
  (if (`KismetStringLibrary.EqualEqual_StrStr` (`self.Name`) "Item")
    (`KismetArrayLibrary.Array_Shuffle` _array)
    (set `self.Name` (`|GetArrayItem` _array (`KismetMathLibrary.RandomIntegerInRange` 0 (- (`KismetArrayLibrary.Array_Length` _array) 1))))))